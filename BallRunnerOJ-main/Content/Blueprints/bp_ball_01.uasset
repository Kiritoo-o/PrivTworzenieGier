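; Rolling ball Blueprint that responds to player input and starts background music on BeginPlay.
; UpDown and LeftRight axes roll the Sphere by applying scaled torque as an acceleration change.
; Space bar restarts a Jumping timeline, which sets the Sphere's height each update by adding a scaled curve offset to the actor's location, with no ground check.
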(event EventBeginPlay
  (Audio|PlaySound2D "/Game/Materials/Elevator_Music__Kevin_MacLeod__-_Gaming_Background_Music__HD_.Elevator_Music__Kevin_MacLeod__-_Gaming_Background_Music__HD_" 1.5 1.0 0.0 0 0))

(event Input|AxisEvents|InputAxisUpDown
  (params (AxisValue :type Float%20%28single-precision%29))
  (Class|PrimitiveComponent|AddTorqueinDegrees (Variables|Default|GetSphere) (Math|Vector|MakeVector 0.0 (* AxisValue (Variables|Default|Getmultiply)) 0.0) "None" true))

(event Input|AxisEvents|InputAxisLeftRight
  (params (AxisValue :type Float%20%28single-precision%29))
  (Class|PrimitiveComponent|AddTorqueinDegrees (Variables|Default|GetSphere) (Math|Vector|MakeVector (* AxisValue (Variables|Default|Getmultiply)) 0.0 0.0) "None" true))

(event Input|KeyboardEvents|SpaceBar
  (params (Key :type Key%20Structure :default "None"))
  (bind _returnvalue (Transformation|GetActorLocation))
  ;[1 1 1] Comment
  (:Pressed
    (bind _jump (Timeline|jumping PlayFromStart)
      (:Update
        (Transformation|SetWorldLocation (Variables|Default|GetSphere) (Math|Vector|MakeVector (.x _returnvalue) (.y _returnvalue) (+ (* (.z _jump) 7.0) (.z _returnvalue))) false false)))))

(fn ConstructionScript)